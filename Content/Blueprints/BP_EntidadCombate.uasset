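; BP_EntidadCombate is a combat entity Blueprint with a world-placed health bar widget.
; One second after BeginPlay, it casts the widget to WBP_BarraVida and passes itself as the entity reference, printing a debug message on success or failure.
; Every tick, it rotates the widget component toward the first player's camera, so the bar acts as a billboard.
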(event EventBeginPlay
  (Utilities|FlowControl|Delay 1.0)
  (bind _aswbp_barra_vida (Utilities|Casting|CastToWBP_BarraVida (UserInterface|GetUserWidgetObject (Variables|Default|GetWidgetBarraVida)))
    (:then
      (Variables|/Game/Interfaces/WBP_BarraVida.WBP_BarraVida_C|SetEntidadReferencia _aswbp_barra_vida self)
      (Development|PrintString "ajuste perfecto" true true "(R=0.000000,G=0.660000,B=1.000000,A=1.000000)" 1e+01))
    (:CastFailed
      (Development|PrintString "falla proyector" true true "(R=0.000000,G=0.660000,B=1.000000,A=1.000000)" 1e+01))))

(event Collision|EventActorBeginOverlap
  (params (OtherActor :type Actor%20Object%20Reference)))

(event EventTick
  (params (DeltaSeconds :type Float%20%28single-precision%29))
  (Transformation|SetWorldRotation (Variables|Default|GetWidgetBarraVida) (Math|Rotator|FindLookatRotation (Transformation|GetWorldLocation (Variables|Default|GetWidgetBarraVida)) (Camera|GetCameraLocation (Game|GetPlayerCameraManager 0))) false false))

(fn ConstructionScript)